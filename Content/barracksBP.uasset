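; Barracks building for an RTS that queues units and releases them at its SpawnLocation socket.
; On spawn it registers its location with TopDownController and creates a SpawnLocation actor.
; PushUnitQueue stores existing unit actors and starts a Delay loop timed by the last queued unit's SpawnTime.
; Each tick of that loop teleports the first unit to the socket, dequeues it and refreshes UI portraits.
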(event `barracksSpawned`
  (bind (_returnvalue_x _returnvalue_y _returnvalue_z) (`KismetMathLibrary.BreakVector` (`self.K2_GetActorLocation`)))
  (bind _output_get (set `self.locationVariable` (`KismetMathLibrary.MakeTransform` (`KismetMathLibrary.MakeVector` _returnvalue_x _returnvalue_y _returnvalue_z))))
  (bind _returnvalue (`GameplayStatics.GetActorOfClass` "/Game/TopDownBP/Blueprints/TopDownController.TopDownController_C"))
  (`KismetArrayLibrary.Array_Append` (`/Game/TopDownBP/Blueprints/TopDownController.ArrayofBuildingLocations` _returnvalue) (`|MakeArray` _output_get))
  (bind _returnvalue_2 (`|SpawnActorFromClass` "/Game/spawnLocation.spawnLocation_C" (`SceneComponent.GetSocketTransform` (`self.Cube`) "SpawnLocation" "RTS_World") "Undefined" "OverrideRootScale" null null))
  (bind _output_get_2 (set `self.spawnLocation` _returnvalue_2)))

(event `spawn unit`)

(event `set timer`
  (bind _arrayofunits (`self.ArrayOfUnits`))
  (bind _returnvalue (`KismetArrayLibrary.Array_LastIndex` _arrayofunits))
  (bind _returnvalue_2 (`KismetMathLibrary.Conv_IntToDouble` (`/Game/enemyType.spawnTime` (`|GetArrayItem` _arrayofunits _returnvalue))))
  (`KismetSystemLibrary.PrintString` (`KismetStringLibrary.Conv_DoubleToString` _returnvalue_2) :!label _label)
  (`KismetSystemLibrary.Delay` _returnvalue_2)
  (`self.PopUnitAndSpawn`)
  (if (> _returnvalue -1)
    (goto _label)))

(fn `getUnitPortraits`
  (for _array_element (`self.ArrayOfUnits`)
    (if (`KismetStringLibrary.Contains` (`KismetSystemLibrary.GetDisplayName` _array_element) "enemy")
      (`KismetArrayLibrary.Array_Add` (`self.UnitPortraits`) (`self.Gun Icon`)))))

(fn `PopUnitAndSpawn`
  (bind _arrayofunits (`self.ArrayOfUnits`))
  (bind _output (`|GetArrayItem` _arrayofunits))
  (bind _cube (`self.Cube`))
  (if (`KismetSystemLibrary.IsValid` _output)
    (`KismetSystemLibrary.PrintString` (`KismetSystemLibrary.GetClassDisplayName` (`GameplayStatics.GetObjectClass` _output)))
    (`self.K2_TeleportTo` (`|GetArrayItem` _arrayofunits) (`SceneComponent.GetSocketLocation` _cube "SpawnLocation") (`SceneComponent.GetSocketRotation` _cube "SpawnLocation"))
    (`KismetArrayLibrary.Array_Remove` _arrayofunits)
    (`/Game/rtsUI_Widget.getIcon` (`/Game/TopDownBP/Blueprints/TopDownCharacter.rts Player UI` (`self.topDownCharacter`)) (`self.Gun Icon`))
    (`/Game/TopDownBP/Blueprints/TopDownController.HideLastIndexPortrait` (`self.topDownController`))
    (`/Game/TopDownBP/Blueprints/TopDownController.DisplayPortraits` (`self.topDownController`))
    (else
      (`KismetSystemLibrary.PrintString` "invalid"))))

(fn `Push Unit Queue`
  (params (UnitToPush :type "/Game/enemyType Object Reference"))
  (`/Engine/EditorBlueprintResources/StandardMacros.IsValid` UnitToPush
    (:`Is Valid`
      (`KismetArrayLibrary.Array_Add` (`self.ArrayOfUnits`) UnitToPush)
      (`KismetSystemLibrary.PrintString` (`KismetSystemLibrary.GetDisplayName` UnitToPush))
      (bind _returnvalue (`GameplayStatics.GetActorOfClass` "/Game/TopDownBP/Blueprints/TopDownCharacter.TopDownCharacter_C"))
      (bind _rts_player_ui (`/Game/TopDownBP/Blueprints/TopDownCharacter.rts Player UI` _returnvalue))
      (for _array_element (`/Game/rtsUI_Widget.BuildIconArray` _rts_player_ui)
        (if (== _array_element "/Game/Textures/gunicon.gunicon")
          (`KismetSystemLibrary.PrintString` "dddddddddddddddddddddddddd")
          (else
            (`KismetSystemLibrary.PrintString` (`KismetSystemLibrary.GetDisplayName` _array_element))
            (`/Game/rtsUI_Widget.getIcon` _rts_player_ui (`self.Gun Icon`))
            (break))))
      (`self.set timer`)
      (`/Game/TopDownBP/Blueprints/TopDownController.DisplayPortraits` (`self.topDownController`)))
    (:`Is Not Valid`
      (`KismetSystemLibrary.PrintString` "invaliddddddddd"))))

(fn `UserConstructionScript`
  (bind _returnvalue (`GameplayStatics.GetActorOfClass` "/Game/TopDownBP/Blueprints/TopDownCharacter.TopDownCharacter_C"))
  (set `self.topDownCharacter` _returnvalue)
  (bind _returnvalue_2 (`GameplayStatics.GetActorOfClass` "/Game/TopDownBP/Blueprints/TopDownController.TopDownController_C"))
  (set `self.topDownController` _returnvalue_2))