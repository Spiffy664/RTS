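; Twin-barrel tower turret that automatically shoots the nearest visible EnemyTest within sensing range.
; Each Tick it picks a target by sphere overlap and line of sight, then rotates its top at constant speed with clamped pitch.
; Once aligned and off cooldown, it fires staggered left/right projectile pairs through a DoN loop, passing on its damage level.
; Upgrade enlarges it and raises damage; touch-to-upgrade and BeginPlay ignore-list setup are disabled.
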(event `self.ReceiveTick`
  (params (DeltaSeconds :type "Float (single-precision)"))
  ;[1 1 1] update turret position, append projectiles to ignore list so the turret won't target it's own projectiles
  (`self.findBestTarget`)
  (`KismetSystemLibrary.PrintString` (`KismetSystemLibrary.GetDisplayName` (`self.Target`)) false)
  (`self.Target`
    (:`then`
      (`self.UpdateTurretRotation` DeltaSeconds)
      (`self.UpdateFire`)
      (bind _outactors (`GameplayStatics.GetAllActorsOfClass` null))
      (`KismetArrayLibrary.Array_Append` (`self.ignoreList`) _outactors))
    (:`else`)))

(event `Fire`
  ;[1 1 1] this is a weird "double shot" which is why it shoots twice and then delays and loops back to keep shooting
  (set `self.TimeOfLastFire` (`KismetSystemLibrary.GetGameTimeInSeconds`))
  (`|ExecutionSequence`
    (:`then_0`
      (goto _label :!via `Reset`))
    (:`then_1`
      (`/Engine/EditorBlueprintResources/StandardMacros.Do N` 2 :!label _label
        (:`Exit`
          (bind _returnvalue (`|SpawnActorFromClass` "/Game/TwinStickBP/Blueprints/TwinStickProjectile.TwinStickProjectile_C" (`SceneComponent.GetSocketTransform` (`self.barrel left`) "BarrelSocket" "RTS_World") "Undefined" "OverrideRootScale" null null))
          (`/Engine/EditorBlueprintResources/StandardMacros.IsValid` _returnvalue
            (:`Is Valid`
              (set `/Game/TwinStickBP/Blueprints/TwinStickProjectile.bulletDamageLevel` (`self.damageLevel`) _returnvalue)
              (`KismetSystemLibrary.Delay` 0.2)
              (bind _returnvalue_2 (`|SpawnActorFromClass` "/Game/TwinStickBP/Blueprints/TwinStickProjectile.TwinStickProjectile_C" (`SceneComponent.GetSocketTransform` (`self.barrelright`) "BarrelSocket" "RTS_World") "Undefined" "OverrideRootScale" null null))
              (`/Engine/EditorBlueprintResources/StandardMacros.IsValid` _returnvalue_2
                (:`Is Valid`
                  (set `/Game/TwinStickBP/Blueprints/TwinStickProjectile.bulletDamageLevel` (`self.damageLevel`) _returnvalue_2)
                  (`KismetSystemLibrary.Delay` 0.2)
                  (goto _label))))))))))

(fn `findBestTarget`
  (locals (`bestDistance(local)` :type "Float (double-precision)") (`currentDistance(local)` :type "Float (double-precision)") (`bestTarget(local)` :type "Actor Object Reference") (`currentTarget(local)` :type "Actor Object Reference"))
  (bind _returnvalue (`self.K2_GetActorLocation`))
  (set `local.bestDistance(local)` (+ (`self.sensingRange(maxDistanceScan)`) 1.0))
  (`KismetSystemLibrary.DrawDebugSphere` _returnvalue)
  (bind _outactors (`KismetSystemLibrary.SphereOverlapActors` _returnvalue (`self.sensingRange(maxDistanceScan)`) (`|MakeArray` "ObjectTypeQuery2" :!type "EObjectTypeQuery Enum") "/Game/TopDownBP/enemyTest.enemyTest_C" (`self.ignoreList`)))
  (for _array_element _outactors
    (bind _output_get (set `local.currentTarget(local)` _array_element))
    (bind _output_get_2 (set `local.currentDistance(local)` (`self.GetDistanceTo` _output_get self)))
    (if (or (< _output_get_2 (`local.bestDistance(local)`)) (not (`KismetSystemLibrary.IsValid` (`local.bestTarget(local)`))))
      (bind _result (`/Game/functionLibrary.hasLineOfSight` (`SceneComponent.K2_GetComponentLocation` (`self.turretTop`)) (`self.K2_GetActorLocation` (`local.currentTarget(local)`)) (`|MakeArray` self (`local.currentTarget(local)`) :!type "Actor Object Reference")))
      (if _result
        (set `local.bestTarget(local)` (`local.currentTarget(local)`))
        (set `local.bestDistance(local)` (`local.currentDistance(local)`)))))
  (set `self.Target` (`local.bestTarget(local)`)))

(fn `UpdateFire`
  (if (> (- (`KismetSystemLibrary.GetGameTimeInSeconds`) (`self.TimeOfLastFire`)) (`self.RateOfFire`))
    (if (> (`KismetMathLibrary.Dot_VectorVector` (`KismetMathLibrary.GetDirectionUnitVector` (`SceneComponent.K2_GetComponentLocation` (`self.turretTop`)) (`self.K2_GetActorLocation` (`self.Target`))) (`SceneComponent.GetForwardVector` (`self.turretTop`))) 0.99)
      (`self.Fire`))))

(fn `UpdateTurretRotation`
  (params (DeltaSeconds :type "Float (double-precision)"))
  (locals (NewRotation :type "Rotator Structure" :default (struct)))
  (bind _output_get (set `local.NewRotation` (`KismetMathLibrary.RInterpTo_Constant` (`SceneComponent.K2_GetComponentRotation` (`self.turretTop`)) (`KismetMathLibrary.FindLookAtRotation` (`SceneComponent.K2_GetComponentLocation` (`self.turretTop`)) (`self.K2_GetActorLocation` (`self.Target`))) (`local.DeltaSeconds`) (`self.RotationSpeed`))))
  (`SceneComponent.K2_SetWorldRotation` (`self.turretTop`) (`KismetMathLibrary.MakeRotator` (.roll _output_get) (`KismetMathLibrary.ClampAngle` (.pitch _output_get) -45.0 75.0) (.yaw _output_get)) false false))

(fn `Upgrade`
  (`self.SetActorScale3D` (1.2 1.2 1.2))
  (`KismetSystemLibrary.PrintString` "Upgraded" false)
  (set `self.damageLevel` 2))

(fn `UserConstructionScript`)